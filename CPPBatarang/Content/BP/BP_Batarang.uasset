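; Batarang actor that plays a start-up sequence with trails, a camera handover and speed UI.
; On BeginPlay it starts two socket-based trails, then after timed delays blends the player's view to itself, adds the speed info widget and sets CanStart on it and the HUD.
; Overlap with BP_Batman only prints a message; the Possess call is disconnected and ChangeLightColor does nothing.
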(event `self.ReceiveBeginPlay`
  (bind _returnvalue (`GameplayStatics.GetPlayerController` 0))
  (`GameplayStatics.GetActorOfClass` (`self.findPlayer`))
  (`ParticleSystemComponent.BeginTrails` (`self.Trail`) "trail" "trail2" "ETrailWidthMode_FromFirst" 0.5)
  (`ParticleSystemComponent.BeginTrails` (`self.TrailRight`) "trail3" "trail4" "ETrailWidthMode_FromFirst" 0.5)
  (`KismetSystemLibrary.Delay` 1.3)
  (`PlayerController.SetViewTargetWithBlend` _returnvalue self 1.0 "VTBlend_Linear" 0.0 false)
  (`KismetSystemLibrary.Delay` 2.0)
  (bind _returnvalue_2 (`|CreateWidget` "/Game/UI/BPW_SpeedInfo.BPW_SpeedInfo_C"))
  (`UserWidget.AddToViewport` _returnvalue_2 0)
  (bind _output_get (set `self.widgetRef` _returnvalue_2))
  (set `/Game/UI/BPW_SpeedInfo.canStart` true _output_get)
  (bind _asbp_hud (cast `/Game/UI/BP_HUD` (`PlayerController.GetHUD` _returnvalue)))
  (set `/Game/UI/BP_HUD.canStart` true _asbp_hud))

(event `EnhancedInput|/Game/Inputs/IA_StopPossess`
  (params (ActionValue :type Boolean) (ElapsedSeconds :type "Float (double-precision)") (TriggeredSeconds :type "Float (double-precision)") (InputAction :type "InputAction Object Reference" :default "/Game/Inputs/IA_StopPossess.IA_StopPossess")))

(event `self.ReceiveActorBeginOverlap`
  (params (OtherActor :type "Actor Object Reference"))
  (cast `/Game/BP/BP_Batman` OtherActor)
  (`KismetSystemLibrary.PrintString` "Now possess"))

(fn `ChangeLightColor`
  (params (lightColor :type "LinearColor Structure")))

(fn `UserConstructionScript`)